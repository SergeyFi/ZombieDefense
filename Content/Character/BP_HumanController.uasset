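; BP_HumanController is a controller that makes the controlled pawn face the point under the mouse cursor.
; It shows the cursor on BeginPlay, then each Tick deprojects the mouse position into a long line trace against WorldStatic objects.
; On a hit, it rotates the pawn using only the look-at yaw, keeping pitch and roll at zero.
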(event `self.ReceiveBeginPlay`
  (set `self.bShowMouseCursor` true))

(event `self.ReceiveTick`
  (params (DeltaSeconds :type "Float (single-precision)"))
  (bind (_worldlocation _worlddirection) (`self.DeprojectMousePositionToWorld`))
  (bind (_outhit _returnvalue) (`KismetSystemLibrary.LineTraceSingleForObjects` _worldlocation (+ (* _worlddirection 50000) _worldlocation) (`|MakeArray` "ObjectTypeQuery1" :!type "EObjectTypeQuery Enum")))
  (if _returnvalue
    (`self.K2_SetActorRotation` (`self.K2_GetPawn`) (`KismetMathLibrary.MakeRotator` 0.0 0.0 (.yaw (`KismetMathLibrary.FindLookAtRotation` (`self.K2_GetActorLocation` (`self.K2_GetPawn`)) (`.Location` (`GameplayStatics.BreakHitResult` _outhit))))) false)))

(fn `UserConstructionScript`)